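; BP_Door is an interactable double sliding door that players open and close.
; Interact plays or reverses DoorTimeline based on IsOpen, sliding Door001 and Door002 apart along local X in mirrored directions.
; An IsAnimating flag blocks input during motion, and IsOpen flips when the timeline finishes.
; CanInteract always allows use, and GetInteractionText returns a Russian open or close prompt matching the current state.
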(event `InteractionInterface.Interact`
  (params (Interactor :type "Actor Object Reference"))
  (if (not (`self.bIsAnimating`))
    (set `self.bIsAnimating` true)
    (if (`self.bIsOpen`)
      (bind (_direction _alpha) (`Timeline|DoorTimeline` :!via `ReverseFromEnd` :!label _label)
        (:`Update`
          (bind _returnvalue (`KismetMathLibrary.MakeVector` (* _alpha 100.0)))
          (`SceneComponent.K2_SetRelativeLocation` (`self.Door_001`) _returnvalue false false)
          (`SceneComponent.K2_SetRelativeLocation` (`self.Door_002`) (* _returnvalue (-1.0 0.0 0.0)) false false))
        (:`Finished`
          (set `self.bIsOpen` (not (`self.bIsOpen`)))
          (set `self.bIsAnimating` false)))
      (else
        (goto _label :!via `PlayFromStart`)))))

(fn `CanInteract`
  (params (Interactor :type "Actor Object Reference"))
  (returns (ReturnValue :type Boolean))
  (return true))

(fn `GetInteractionText`
  (returns (ReturnValue :type Text))
  (if (`self.bIsOpen`)
    (return "Закрыть")
    (else
      (return "Открыть"))))

(fn `UserConstructionScript`)