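; Held flashlight item from the inventory system, attached to the right-hand socket, that lets the player switch a spotlight on and off.
; Using it flips the On state, applies it to the SpotLight's visibility and plays a 2D click sound.
; Equipping syncs the light to the On state, and unequipping resets that state to off without updating the light itself.
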(event `HoldableInterface.OnEquipped`
  (params (Holder :type "Actor Object Reference"))
  (`SceneComponent.SetVisibility` (`self.SpotLight`) (`self.bOn`) false))

(event `HoldableInterface.OnHeldUse`
  (bind _output_get (set `self.bOn` (not (`self.bOn`))))
  (`SceneComponent.SetVisibility` (`self.SpotLight`) _output_get false)
  (`GameplayStatics.PlaySound2D` "/Game/Inventory/Flashlight/502506__rudmer_rotteveel__small_flashlight_click_on_fast.502506__rudmer_rotteveel__small_flashlight_click_on_fast" 1.0 1.0 0.0 null null))

(event `HoldableInterface.OnUnEquipped`
  (set `self.bOn` false))

(fn `GetHandSocket`
  (returns (ReturnValue :type Name))
  (return "hand_r"))

(fn `UserConstructionScript`)