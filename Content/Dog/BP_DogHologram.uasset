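; BP_DogHologram is an interactable dog hologram that spins and plays a voice or audio clip when used.
; Tick yaws the Dog component at a frame-rate-independent rate set by Speed.
; Interact plays the Ecliptor_prolog sound as non-spatial 2D audio, with no guard against repeat triggering.
; CanInteract always allows interaction, and GetInteractionText returns an empty prompt.
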(event `self.ReceiveTick`
  (params (DeltaSeconds :type "Float (single-precision)"))
  (`SceneComponent.K2_AddLocalRotation` (`self.dog`) (`KismetMathLibrary.MakeRotator` 0.0 0.0 (* DeltaSeconds (`self.Speed`))) false false))

(event `InteractionInterface.Interact`
  (params (Interactor :type "Actor Object Reference"))
  (`GameplayStatics.PlaySound2D` "/Game/Sounds/ecliptor_prolog.ecliptor_prolog" 1.0 1.0 0.0 null null))

(fn `CanInteract`
  (params (Interactor :type "Actor Object Reference"))
  (returns (ReturnValue :type Boolean))
  (return true))

(fn `GetInteractionText`
  (returns (ReturnValue :type Text))
  (return ""))

(fn `UserConstructionScript`)